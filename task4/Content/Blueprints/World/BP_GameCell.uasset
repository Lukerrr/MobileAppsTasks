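; Clickable, touchable cell for a color-matching grid puzzle, colored by CellClass through a dynamic material.
; Row and column come from attachment order within parent stacks, and active cells interpolate toward their row's height each tick.
; A tap with same-class orthogonal neighbors triggers a recursive flood fill, using IsActive to prevent revisits.
; Each removed cell notifies its BP_CellStack, then gets launched with physics force and torque.
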(event `self.ReceiveTick`
  (params (DeltaSeconds :type "Float (single-precision)"))
  (if (`self.bIsActive`)
    (bind _asbp_game_state (cast `/Game/Blueprints/System/BP_GameState` (`GameplayStatics.GetGameState`)))
    (`self.K2_SetActorRelativeLocation` (`KismetMathLibrary.VInterpTo` (`KismetMathLibrary.MakeVector` 0.0 0.0 (`self.GetCellHeight`)) (`KismetMathLibrary.MakeVector` 0.0 0.0 (* (+ (`self.GetRow`) 1) (`/Game/Blueprints/World/BP_GameField.CellSpacing` (`/Game/Blueprints/System/BP_GameState.GetGameField` _asbp_game_state)))) (`GameplayStatics.GetWorldDeltaSeconds`) 5.0))))

(event `RequestDestroyCell`
  (bind _result (`self.CanBeDestroyed`))
  (if _result
    (bind _neighbors (`self.FindNeighbors`))
    (set `self.bIsActive` false)
    (for _array_element _neighbors
      (`self.RequestDestroyCell` _array_element))
    (`self.DestroyCell`)))

(event `self.StaticMesh.OnClicked`
  (params (TouchedComponent :type "PrimitiveComponent Object Reference") (ButtonPressed :type "Key Structure"))
  (`self.RequestDestroyCell`))

(event `self.StaticMesh.OnInputTouchBegin`
  (params (FingerIndex :type "ETouchIndex Enum" :default "Touch1") (TouchedComponent :type "PrimitiveComponent Object Reference"))
  (`self.RequestDestroyCell`))

(fn `CanBeDestroyed`
  (returns (Result :type Boolean))
  (if (`self.bIsActive`)
    (bind _neighbors (`self.FindNeighbors`))
    (return (> (`KismetArrayLibrary.Array_Length` _neighbors) 0))
    (else
      (return false))))

(fn `DestroyCell`
  (bind _staticmesh (`self.StaticMesh`))
  (`/Game/Blueprints/World/BP_CellStack.OnCellDestroyed` (`self.GetParentStack`) self)
  (`PrimitiveComponent.SetSimulatePhysics` _staticmesh true)
  (`PrimitiveComponent.AddForce` _staticmesh (65000.0 0.0 0.0) "None" true)
  (`PrimitiveComponent.AddTorqueInRadians` _staticmesh (0.0 1000.0 0.0) "None" true))

(fn `FindNeighbors`
  (returns (Neighbors :type "Array of /Game/Blueprints/World/BP_GameCell Object Reference"))
  (locals (Result :type "Array of /Game/Blueprints/World/BP_GameCell Object Reference"))
  (bind _row (`self.GetRow`))
  (bind _column (`self.GetColumn`))
  (bind _result (`local.Result`))
  (`|ExecutionSequence`
    (:`then_0`
      (`self.ValidateNeighbor` (- _row 1) _column _result))
    (:`then_1`
      (`self.ValidateNeighbor` (+ _row 1) _column _result))
    (:`then_2`
      (`self.ValidateNeighbor` _row (- _column 1) _result))
    (:`then_3`
      (`self.ValidateNeighbor` _row (+ _column 1) _result))
    (:`then_4`
      (return (`local.Result`)))))

(fn `GetCellHeight`
  (returns (Height :type "Float (double-precision)"))
  (bind (_returnvalue_x _returnvalue_y _returnvalue_z) (`KismetMathLibrary.BreakVector` (- (`self.K2_GetActorLocation`) (`self.K2_GetActorLocation` (`self.GetAttachParentActor`)))))
  (return _returnvalue_z))

(fn `GetColumn`
  (returns (Column :type Integer))
  (bind _returnvalue (`self.GetAttachParentActor`))
  (return (`KismetArrayLibrary.Array_Find` (`self.GetAttachedActors` (`self.GetAttachParentActor` _returnvalue) false) _returnvalue)))

(fn `GetParentStack`
  (returns (Stack :type "/Game/Blueprints/World/BP_CellStack Object Reference"))
  (bind _asbp_cell_stack (cast `/Game/Blueprints/World/BP_CellStack` (`self.GetAttachParentActor`)))
  (return _asbp_cell_stack))

(fn `GetRow`
  (returns (Row :type Integer))
  (return (`KismetArrayLibrary.Array_Find` (`self.GetAttachedActors` (`self.GetAttachParentActor`) false) self)))

(fn `UserConstructionScript`
  (bind _returnvalue (`PrimitiveComponent.CreateDynamicMaterialInstance` (`self.StaticMesh`) 0 "/Game/Materials/Mat_Cube.Mat_Cube" "None"))
  (`MaterialInstanceDynamic.SetVectorParameterValue` _returnvalue "GlowColor" (select `int` (`self.CellClass`) :`0` (struct :`R` 1.0 :`G` 0.09097 :`B` 0.051168 :`A` 1.0) :`1` (struct :`R` 0.096735 :`G` 0.614583 :`A` 1.0) :`2` (struct :`G` 0.243414 :`B` 1.0 :`A` 1.0) :!type "LinearColor Structure")))