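; Game state for a grid-based cell-clearing puzzle that restarts the game, looks up cells and detects victory or defeat.
; Restarting destroys all cells and stacks, then has BP_GameField regenerate; FindGameCell resolves row and column through its attached-actor hierarchy.
; Cell destruction sets a flag that defers checking to Tick.
; No active cells means victory and no destroyable cells means defeat, either showing the restart widget.
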(event `self.ReceiveBeginPlay`
  (`self.RestartGame`))

(event `self.ReceiveTick`
  (params (DeltaSeconds :type "Float (single-precision)"))
  (if (`self.bCheckAvailableCells`)
    (set `self.bCheckAvailableCells` false)
    (`self.CheckCells`)))

(event `OnGameCellDestroyed`
  (if (`self.bIsGameActive`)
    (set `self.bCheckAvailableCells` true)))

(fn `CheckCells`
  (bind _gamefield (`self.GetGameField`))
  (bind _result (`/Game/Blueprints/World/BP_GameField.HasActiveCells` _gamefield))
  (if _result
    (bind _result_2 (`/Game/Blueprints/World/BP_GameField.HasDestroyableCells` _gamefield))
    (if (not _result_2)
      (`self.StopGame` false))
    (else
      (`self.StopGame` true))))

(fn `FindGameCell`
  (params (Row :type Integer) (Column :type Integer))
  (returns (Cell :type "/Game/Blueprints/World/BP_GameCell Object Reference"))
  (locals (Columns :type "Array of Actor Object Reference") (Rows :type "Array of Actor Object Reference"))
  (`|ExecutionSequence`
    (:`then_0`
      (if (or (< (`local.Row`) 0) (< (`local.Column`) 0))
        (return null)))
    (:`then_1`
      (set `local.Columns` (`self.GetAttachedActors` (`self.GetGameField`) true)))
    (:`then_2`
      (if (>= (`local.Column`) (`KismetArrayLibrary.Array_Length` (`local.Columns`)))
        (return null)))
    (:`then_3`
      (set `local.Rows` (`self.GetAttachedActors` (`|GetArrayItem` (`local.Columns`) (`local.Column`)) true)))
    (:`then_4`
      (if (>= (`local.Row`) (`KismetArrayLibrary.Array_Length` (`local.Rows`)))
        (return null)))
    (:`then_5`
      (bind _asbp_game_cell (cast `/Game/Blueprints/World/BP_GameCell` (`|GetArrayItem` (`local.Rows`) (`local.Row`)))
        (:`then`
          (return _asbp_game_cell))
        (:`CastFailed`
          (return null))))))

(fn `GetGameField`
  (returns (GameField :type "/Game/Blueprints/World/BP_GameField Object Reference"))
  (bind _returnvalue (`GameplayStatics.GetActorOfClass` "/Game/Blueprints/World/BP_GameField.BP_GameField_C"))
  (return _returnvalue))

(fn `RestartGame`
  (bind _outactors (`GameplayStatics.GetAllActorsOfClass` "/Game/Blueprints/World/BP_GameCell.BP_GameCell_C"))
  (for _array_element _outactors
    (`self.K2_DestroyActor` _array_element))
  (bind _outactors_2 (`GameplayStatics.GetAllActorsOfClass` "/Game/Blueprints/World/BP_CellStack.BP_CellStack_C"))
  (for _array_element_2 _outactors_2
    (`self.K2_DestroyActor` _array_element_2))
  (`/Game/Blueprints/World/BP_GameField.GenerateField` (`self.GetGameField`))
  (set `self.bIsGameActive` true)
  (`self.CheckCells`))

(fn `StopGame`
  (params (bVictory :type Boolean))
  (set `self.bIsGameActive` false)
  (bind _returnvalue (`|CreateWidget` "/Game/Blueprints/Widgets/BP_RestartWidget.BP_RestartWidget_C" (`GameplayStatics.GetPlayerController` 0) bVictory))
  (`UserWidget.AddToViewport` _returnvalue 0))

(fn `UserConstructionScript`)